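; BP_CanGoInBasement is an actor that unlocks the basement once the player's key story items are found.
; Each Tick it checks the game instance's Book, Drawing3 and Necklace flags and fires a single DoOnce when all three are set.
; After a short delay it sets HasKey on the first-person character, plays a door-opening sound at a scene component, and shows an unlock prompt.
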(event `self.ReceiveTick`
  (params (DeltaSeconds :type "Float (single-precision)"))
  (bind _asgi_horror_game (cast `/Game/Sebastian/GI_HorrorGame` (`GameplayStatics.GetGameInstance`)))
  (if (and (`/Game/Sebastian/GI_HorrorGame.Book` _asgi_horror_game) (`/Game/Sebastian/GI_HorrorGame.Drawing3` _asgi_horror_game) (`/Game/Sebastian/GI_HorrorGame.Necklace` _asgi_horror_game))
    (`/Engine/EditorBlueprintResources/StandardMacros.DoOnce` false
      (:`Completed`
        (`KismetSystemLibrary.Delay` 5.0)
        (bind _asbp_first_person_character (cast `/Game/FirstPerson/Blueprints/BP_FirstPersonCharacter` (`GameplayStatics.GetPlayerCharacter` 0)))
        (set `/Game/FirstPerson/Blueprints/BP_FirstPersonCharacter.HasKey` true _asbp_first_person_character)
        (`GameplayStatics.PlaySoundAtLocation` "/Game/Sebastian/sounds1/S2/OpenDoorBasement.OpenDoorBasement" (`SceneComponent.K2_GetComponentLocation` (`self.SounddOrigin`)) (struct) 1.0 1.0 0.0 null null null null)
        (`KismetSystemLibrary.Delay` 1.0)
        (`/Game/Sebastian/MainMenu/InGame/BPL_UI.Show in Game Prompt` "Sounds like a door unlocked.")))))

(fn `UserConstructionScript`)