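; Placeable nightstand (Nachtisch) with a drawer that opens and closes on Interact, with a sound for each direction.
; The GoOut timeline slides the component passed to Interact along its relative X axis, playing forward to open and reversed to close.
; Two cross-reset DoOnce gates form a toggle that ignores input mid-motion: fully open arms closing, fully closed re-arms opening.
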(event `/Game/FirstPerson/Blueprints/BPI_Interact.Interact`
  (params (ActorComponent :type "SceneComponent Object Reference"))
  (`|ExecutionSequence`
    (:`then_0`
      (`/Engine/EditorBlueprintResources/StandardMacros.DoOnce` false :!label _label
        (:`Completed`
          (`GameplayStatics.PlaySound2D` "/Game/Sebastian/sounds1/s3/Furniture/Drawer_Open_22.Drawer_Open_22" 1.0 1.0 0.0 null null)
          (bind (_direction _alha) (`Timeline|GoOut` :!via `PlayFromStart` :!label _label_2)
            (:`Update`
              (`SceneComponent.K2_SetRelativeLocation` ActorComponent (`KismetMathLibrary.MakeVector` (`KismetMathLibrary.Lerp` 0.0 20.0 _alha)) false false))
            (:`Finished`
              (switch `ETimelineDirection` _direction
                (:`Forward`
                  (goto _label_3 :!via `Reset`))
                (:`Backward`
                  (goto _label :!via `Reset`))))))))
    (:`then_1`
      (`/Engine/EditorBlueprintResources/StandardMacros.DoOnce` true :!label _label_3
        (:`Completed`
          (`GameplayStatics.PlaySound2D` "/Game/Sebastian/sounds1/S2/Furniture/Drawer_Close_23.Drawer_Close_23" 1.0 1.0 0.0 null null)
          (goto _label_2 :!via `Reverse`))))))

(fn `Interact Result`
  (params (HitResult :type "HitResult Structure"))
  (return))

(fn `UserConstructionScript`)