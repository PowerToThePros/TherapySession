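; Left cabinet door (SchranktuerLinks) that swings open and closed when interacted with.
; Interact toggles on the Open flag, playing a drawer sound and running the Move timeline forward or in reverse.
; The timeline lerps the Scene component's relative yaw between zero and Rotation.
; Two DoOnce gates, reset when the timeline finishes in each direction, block re-triggering mid-swing, and Open clears only once fully closed.
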(event `/Game/FirstPerson/Blueprints/BPI_Interact.Interact`
  (params (ActorComponent :type "SceneComponent Object Reference"))
  (if (`self.Open`)
    (`/Engine/EditorBlueprintResources/StandardMacros.DoOnce` false :!label _label
      (:`Completed`
        (`GameplayStatics.PlaySound2D` "/Game/Sebastian/sounds1/s3/Furniture/Drawer_Close_23.Drawer_Close_23" 1.0 1.0 0.0 null null)
        (bind (_direction _alpha) (`Timeline|Move` :!via `Reverse` :!label _label_2)
          (:`Update`
            (`SceneComponent.K2_SetRelativeRotation` (`self.Scene`) (`KismetMathLibrary.MakeRotator` 0.0 0.0 (`KismetMathLibrary.Lerp` 0.0 (`self.Rotation`) _alpha)) false false))
          (:`Finished`
            (switch `ETimelineDirection` _direction
              (:`Forward`
                (goto _label :!via `Reset`))
              (:`Backward`
                (set `self.Open` false)
                (goto _label_3 :!via `Reset`)))))))
    (else
      (set `self.Open` true)
      (`/Engine/EditorBlueprintResources/StandardMacros.DoOnce` false :!label _label_3
        (:`Completed`
          (`GameplayStatics.PlaySound2D` "/Game/Sebastian/sounds1/s3/Furniture/Drawer_Open_22.Drawer_Open_22" 1.0 1.0 0.0 null null)
          (goto _label_2 :!via `PlayFromStart`))))))

(fn `UserConstructionScript`)