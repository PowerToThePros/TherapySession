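; Interactable dining room light that toggles between on and off when the player interacts with it.
; Interact branches on IsOn through two DoOnce gates that re-arm each other, playing the matching switch sound.
; CanTurnOn gates the actual change of spot light visibility and emissive or plastic mesh material, though the sound plays regardless.
; The construction script applies the initial IsOn state to light and material.
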(event `/Game/FirstPerson/Blueprints/BPI_Interact.Interact`
  (params (ActorComponent :type "SceneComponent Object Reference"))
  (if (`self.IsOn`)
    (`/Engine/EditorBlueprintResources/StandardMacros.DoOnce` false :!label _label
      (:`Completed`
        (`GameplayStatics.PlaySoundAtLocation` "/Game/Sebastian/sounds1/S2/light/LightOff.LightOff" (`self.K2_GetActorLocation`) (struct) 1.0 1.0 0.0 null null null null)
        (if (`self.CanTurnOn`)
          (`SceneComponent.SetVisibility` (`self.SpotLight`) false false)
          (`PrimitiveComponent.SetMaterial` (`self.StaticMesh`) 0 "/Game/Marvin/Materials/MI_Plastik.MI_Plastik")
          (set `self.IsOn` false)
          (goto _label_2 :!via `Reset`)
          (else
            (goto _label :!via `Reset`)))))
    (else
      (`/Engine/EditorBlueprintResources/StandardMacros.DoOnce` false :!label _label_2
        (:`Completed`
          (`GameplayStatics.PlaySoundAtLocation` "/Game/Sebastian/sounds1/S2/light/LightOn.LightOn" (`self.K2_GetActorLocation`) (struct) 1.0 1.0 0.0 null null null null)
          (if (`self.CanTurnOn`)
            (`SceneComponent.SetVisibility` (`self.SpotLight`) true false)
            (`PrimitiveComponent.SetMaterial` (`self.StaticMesh`) 0 "/Game/Marvin/Materials/MI_Emissiv_Yellow_ON.MI_Emissiv_Yellow_ON")
            (set `self.IsOn` true)
            (goto _label :!via `Reset`)
            (else
              (goto _label_2 :!via `Reset`))))))))

(fn `UserConstructionScript`
  (bind _ison (`self.IsOn`))
  (`SceneComponent.SetVisibility` (`self.SpotLight`) _ison false)
  (if _ison
    (`PrimitiveComponent.SetMaterial` (`self.StaticMesh`) 0 "/Game/Marvin/Materials/MI_Emissiv_Yellow_ON.MI_Emissiv_Yellow_ON")
    (else
      (`PrimitiveComponent.SetMaterial` (`self.StaticMesh`) 0 "/Game/Marvin/Materials/MI_Plastik.MI_Plastik"))))