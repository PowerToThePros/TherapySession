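; BP_Day3 is an interactable actor that triggers the game's ending once four collectibles are flagged in GI_HorrorGame: Drawing3, PictureOfAva, Book and Necklace.
; Tick polls those flags and, once all are set, shows an in-game prompt a single time after a delay.
; Interact repeats the check, then once plays a level sequence, destroys the player character and opens the end credits level after a timed delay.
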(event `self.ReceiveTick`
  (params (DeltaSeconds :type "Float (single-precision)"))
  (bind _asgi_horror_game (cast `/Game/Sebastian/GI_HorrorGame` (`GameplayStatics.GetGameInstance`)))
  (if (and (`/Game/Sebastian/GI_HorrorGame.Drawing3` _asgi_horror_game) (`/Game/Sebastian/GI_HorrorGame.PictureOfAva` _asgi_horror_game) (`/Game/Sebastian/GI_HorrorGame.Book` _asgi_horror_game) (`/Game/Sebastian/GI_HorrorGame.Necklace` _asgi_horror_game))
    (`/Engine/EditorBlueprintResources/StandardMacros.DoOnce` false
      (:`Completed`
        (`KismetSystemLibrary.Delay` 7.0)
        (`/Game/Sebastian/MainMenu/InGame/BPL_UI.Show in Game Prompt` (`self.DisplayText`))))))

(event `/Game/FirstPerson/Blueprints/BPI_Interact.Interact`
  (params (ActorComponent :type "SceneComponent Object Reference"))
  (bind _asgi_horror_game (cast `/Game/Sebastian/GI_HorrorGame` (`GameplayStatics.GetGameInstance`)))
  (if (and (`/Game/Sebastian/GI_HorrorGame.Drawing3` _asgi_horror_game) (`/Game/Sebastian/GI_HorrorGame.PictureOfAva` _asgi_horror_game) (`/Game/Sebastian/GI_HorrorGame.Book` _asgi_horror_game) (`/Game/Sebastian/GI_HorrorGame.Necklace` _asgi_horror_game))
    (`/Engine/EditorBlueprintResources/StandardMacros.DoOnce` false
      (:`Completed`
        (`MovieSceneSequencePlayer.Play` (`LevelSequenceActor.SequencePlayer` (`self.sequence`)))
        (`self.K2_DestroyActor` (`GameplayStatics.GetPlayerCharacter` 0))
        (`KismetSystemLibrary.Delay` 7.3)
        (`GameplayStatics.OpenLevelBySoftObjectPtr` "/Game/Sebastian/MainMenu/EndCredits.EndCredits")))))

(fn `UserConstructionScript`)