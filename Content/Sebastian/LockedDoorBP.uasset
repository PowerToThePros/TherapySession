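; An interactable door Blueprint that can require the player to hold a key, playing a rate-limited locked sound without one.
; A dot product against the player's position picks the swing direction, and a Timeline curve rotates the mesh up to 90 degrees.
; DoOnce gates let a later interaction reverse the Timeline to close it.
; The construction script sets the starting Timeline time and swing side from editable variables.
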(event `self.ReceiveBeginPlay`
  (bind _asbp_first_person_character (cast `/Game/FirstPerson/Blueprints/BP_FirstPersonCharacter` (`GameplayStatics.GetPlayerCharacter` 0)))
  (set `self.PlayerRef` _asbp_first_person_character))

(event `/Game/FirstPerson/Blueprints/BPI_Interact.Interact`
  (params (ActorComponent :type "SceneComponent Object Reference"))
  (if (`self.NeedKey`)
    (bind _asbp_first_person_character (cast `/Game/FirstPerson/Blueprints/BP_FirstPersonCharacter` (`GameplayStatics.GetPlayerCharacter` 0)))
    (if (`/Game/FirstPerson/Blueprints/BP_FirstPersonCharacter.HasKey` _asbp_first_person_character)
      (`/Engine/EditorBlueprintResources/StandardMacros.DoOnce` false :!label _label
        (:`Completed`
          (`self.OpenDoor`)))
      (elif (`self.CanPlaySoundAgain`)
        (set `self.CanPlaySoundAgain` false)
        (`GameplayStatics.PlaySoundAtLocation` "/Game/StarterContent/Audio/Collapse01.Collapse01" (`self.K2_GetActorLocation`) (struct) 1.0 1.0 0.0 null null null null)
        (`KismetSystemLibrary.Delay` (`self.DoorSoundDelay`))
        (set `self.CanPlaySoundAgain` true)))
    (else
      (goto _label))))

(event `OpenDoor`
  (bind _returnvalue (`self.K2_GetActorLocation`))
  (bind _scene (`self.Scene`))
  (if (`self.IsDoorClosed`)
    (set `self.IsDoorClosed` false)
    (set `self.DotProduct` (`KismetMathLibrary.Dot_VectorVector` (`KismetMathLibrary.Normal` (- (`SceneComponent.K2_GetComponentLocation` _scene) (`self.K2_GetActorLocation` (`self.PlayerRef`)))) (`SceneComponent.GetForwardVector` _scene)))
    (`GameplayStatics.PlaySoundAtLocation` "/Game/FPWeapon/Audio/FirstPersonTemplateWeaponFire02.FirstPersonTemplateWeaponFire02" _returnvalue (struct) 1.0 1.0 0.0 null null null null)
    (bind (_direction _doorcurve) (`Timeline|DoorAnim` :`NewTime` (stale `UpdateDoorRotation` NewTime) :!label _label_2)
      (:`Update`
        (`SceneComponent.K2_SetRelativeRotation` (`self.MeshRoot`) (`KismetMathLibrary.MakeRotator` 0.0 0.0 (`KismetMathLibrary.Lerp` 0.0 (`KismetMathLibrary.SelectFloat` 90.0 -90.0 (>= (`self.DotProduct`) 0.0)) _doorcurve)) false false))
      (:`Finished`
        (`|ExecutionSequence`
          (:`then_0`
            (goto _label :!via `Reset`))
          (:`then_1`
            (switch `ETimelineDirection` _direction
              (:`Forward`
                (goto _label_3 :!via `Reset`))
              (:`Backward`
                (set `self.IsDoorClosed` true)))))))
    (else
      (`/Engine/EditorBlueprintResources/StandardMacros.DoOnce` false :!label _label_3
        (:`Completed`
          (`GameplayStatics.PlaySoundAtLocation` "/Game/StarterContent/Audio/Explosion01.Explosion01" _returnvalue (struct) 1.0 1.0 0.0 null null null null)
          (goto _label_2 :!via `Reverse`))))))

(event `UpdateDoorRotation`
  (params (NewTime :type "Float (single-precision)") (DotProduct :type "Float (double-precision)"))
  (set `self.DotProduct` DotProduct)
  (goto _label_2 :!via `SetNewTime`))

(fn `UserConstructionScript`
  (`self.UpdateDoorRotation` (`self.DoorStartRotation`) (select `bool` (`self.FlipDoor`) :`false` 45.0 :`true` -45.0)))